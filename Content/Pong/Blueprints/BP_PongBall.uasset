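; BP_PongBall is the ball for a Pong game, launched in a random direction when play begins.
; On BeginPlay, a coin flip picks one of two yaw ranges and a random yaw is clamped into it, keeping the heading away from the zero and 180-degree axis.
; The actor rotates to that yaw, then its Sphere gets a fixed physics linear velocity along the forward vector.
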(event EventBeginPlay
  (if (Math|Random|RandomBool)
    (Variables|Default|SetClamp%20Rotation (Math|Float|Clamp(Float) (.yaw (Math|Random|RandomRotator false)) 2e+01 1.6e+02))
    (else
      (Variables|Default|SetClamp%20Rotation (Math|Float|Clamp(Float) (.yaw (Math|Random|RandomRotator false)) 2.1e+02 3.4e+02))))
  (Transformation|SetActorRotation (Math|Rotator|MakeRotator 0.0 0.0 (Variables|Default|GetClamp%20Rotation)))
  (Physics|SetPhysicsLinearVelocity (Variables|Default|GetSphere) (* (Transformation|GetActorForwardVector) (Math|Float|MakeLiteralFloat 2.5e+03)) false "None"))

(fn ConstructionScript)