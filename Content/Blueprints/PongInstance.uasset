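; PongInstance keeps the left and right scores for a Pong game.
; Its AddScore event uses a boolean to choose a side and adds the given points to that side's running total.
; It then prints both totals as one string with no separator between them.
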(event Custom|AddScore
  (params (Points :type Integer) (LeftScore :type Boolean))
  (if LeftScore
    (Variables|Default|SetLeftScore (+ (Variables|Default|GetLeftScore) Points))
    (else
      (Variables|Default|SetRightScore (+ (Variables|Default|GetRightScore) Points))))
  (Development|PrintString (Utilities|String|Append (Utilities|String|ToString(Integer) (Variables|Default|GetLeftScore)) (Utilities|String|ToString(Integer) (Variables|Default|GetRightScore)))))